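; Player inventory component for a Zelda-style game, also handling rupees, health and the related widgets.
; A per-tick sphere trace at the player's feet finds collectables for the interact input, while capsule overlaps collect rupees.
; Weapons and shields fill fixed slots and auto-equip when none is equipped; materials stack to DataTable limits in a growable array.
; It also drops and spawns items, and swaps adjacent slots by quantity when the inventory closes.
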(event `self.ReceiveBeginPlay`
  (bind (_weapons _shields) (break `/Game/Items/S_InventoryItems` (`self.InventoryItems`)))
  (`EnhancedInputSubsystemInterface.AddMappingContext` (pcsubsystem `EnhancedInputLocalPlayerSubsystem` (`GameplayStatics.GetPlayerController` 0)) "/Game/Inputs/IMC_Zelda.IMC_Zelda" 0 (struct))
  (bind _returnvalue (`|CreateWidget` "/Game/Widgets/WBP_Inventory.WBP_Inventory_C"))
  (set `self.WBP_InventoryWidget` _returnvalue)
  (bind _asbp_third_person_character (cast `/Game/ThirdPerson/Blueprints/BP_ThirdPersonCharacter` (`GameplayStatics.GetPlayerCharacter` 0)))
  (bind _output_get (set `self.ThirdPersonCharacter` _asbp_third_person_character))
  (add `PrimitiveComponent.OnComponentBeginOverlap` (`Character.CapsuleComponent` _output_get) (`|CreateDelegate` :!event `PickUpRupee`))
  (`self.InitHealthBar`)
  (bind _returnvalue_2 (`|CreateWidget` "/Game/Widgets/WBP_Interact.WBP_Interact_C"))
  (set `self.WBP_Interact` _returnvalue_2)
  (`KismetArrayLibrary.Array_Resize` _weapons 5)
  (`KismetArrayLibrary.Array_Resize` _shields 5)
  (`/Game/Widgets/WBP_Inventory.Reset Items UI In Inventory` (`self.WBP_InventoryWidget`))
  (bind _returnvalue_3 (`|CreateWidget` "/Game/Widgets/WBP_ItemWarning.WBP_ItemWarning_C"))
  (bind _output_get_2 (set `self.WBP_ItemWarning` _returnvalue_3))
  (`UserWidget.AddToViewport` _output_get_2 0))

(event `self.ReceiveTick`
  (params (DeltaSeconds :type "Float (single-precision)"))
  (bind (_found _founditem _itemactor) (`self.TraceItemToPickUp`))
  (if _found
    (if (`Widget.IsInViewport` (`self.WBP_Interact`))
      (if (not (== _itemactor (`self.FoundItem`)))
        (set `self.FoundItem` _itemactor :!label _label))
      (else
        (`UserWidget.AddToViewport` (`self.WBP_Interact`) 0)
        (goto _label)))
    (elif (`Widget.IsInViewport` (`self.WBP_Interact`))
      (`Widget.RemoveFromParent` (`self.WBP_Interact`))
      (set `self.FoundItem` null))))

(event `EnhancedInput|/Game/Inputs/IA_Inventory`
  (params (ActionValue :type Boolean) (ElapsedSeconds :type "Float (double-precision)") (TriggeredSeconds :type "Float (double-precision)") (InputAction :type "InputAction Object Reference" :default "/Game/Inputs/IA_Inventory.IA_Inventory"))
  (bind _returnvalue (`GameplayStatics.GetPlayerController` 0))
  (:`Triggered`
    (`self.OnInventoryOpen`)
    (`GameplayStatics.SetGamePaused` true)
    (set `PlayerController.bShowMouseCursor` true _returnvalue)
    (`WidgetBlueprintLibrary.SetInputMode_UIOnlyEx` _returnvalue (`self.WBP_InventoryWidget`))
    (`/Game/Widgets/WBP_Inventory.Reset Items UI In Inventory` (`self.WBP_InventoryWidget`))))

(event `EnhancedInput|/Game/Inputs/IA_InteractWithItem`
  (params (ActionValue :type Boolean) (ElapsedSeconds :type "Float (double-precision)") (TriggeredSeconds :type "Float (double-precision)") (InputAction :type "InputAction Object Reference" :default "/Game/Inputs/IA_InteractWithItem.IA_InteractWithItem"))
  (:`Triggered`
    (if (`KismetSystemLibrary.IsValid` (`self.FoundItem`))
      (bind _asbp_collectable_item (cast `/Game/Items/Collectatbles/BP_CollectableItem` (`self.FoundItem`)))
      (bind _item (`/Game/Items/Collectatbles/BP_CollectableItem.Item` _asbp_collectable_item))
      (bind (_itemid _quantity _itemtype) (break `/Game/Items/Collectatbles/S_Slot` _item))
      (switch `/Game/Enums/EnumItemType` _itemtype
        (:`NewEnumerator0`
          (bind _add_to_inventory_successful (`self.AddToInventory` _item (`.Materials_11_A4C8D597405D82D79F98BAA9BD1B6C02` (break `/Game/Items/S_InventoryItems` (`self.InventoryItems`)))))
          (if _add_to_inventory_successful
            (`Actor.K2_DestroyActor` (`self.FoundItem`) :!label _label)
            (`/Game/Widgets/WBP_Inventory.Reset Items UI In Inventory` (`self.WBP_InventoryWidget`))
            (else
              (`KismetSystemLibrary.PrintString` "You can not add any more of this item" :!label _label_2)
              (`/Game/Widgets/WBP_ItemWarning.ActivateWarning` (`self.WBP_ItemWarning`) _itemtype))))
        (:`NewEnumerator1`
          (bind _add_to_inventory_successful_2 (`self.AddToInventory` _item (`.Weapons_6_204640D1462B9325452B4492E2270A77` (break `/Game/Items/S_InventoryItems` (`self.InventoryItems`)))))
          (if _add_to_inventory_successful_2
            (goto _label)
            (else
              (goto _label_2))))
        (:`NewEnumerator2`
          (bind _add_to_inventory_successful_3 (`self.AddToInventory` _item (`.Shields_9_97E983774B854D39919EFCBD26DFE85F` (break `/Game/Items/S_InventoryItems` (`self.InventoryItems`)))))
          (if _add_to_inventory_successful_3
            (goto _label)
            (else
              (goto _label_2))))))))

(fn `AddToInventory`
  (params (Item :type "/Game/Items/Collectatbles/S_Slot Structure") (ItemArray :type "Array of /Game/Items/Collectatbles/S_Slot Structure"))
  (returns (`Add To Inventory Successful` :type Boolean))
  (locals (Index :type Integer))
  (bind _item (`local.Item`))
  (bind (_itemid _quantity _itemtype) (break `/Game/Items/Collectatbles/S_Slot` (`local.Item`)))
  (for (_array_element _array_index) ItemArray
    (set `local.Index` _array_index)
    (bind (_itemid_2 _quantity_2) (break `/Game/Items/Collectatbles/S_Slot` _array_element))
    (bind (_datatable _rowname) (break `DataTableRowHandle` _itemid_2))
    (if (== _rowname "None")
      (`KismetArrayLibrary.Array_Set` (`local.ItemArray`) (`local.Index`) _item)
      (switch `/Game/Enums/EnumItemType` (`.ItemType_9_26E7E05B4F92E22B1DD70092B75988D9` (break `/Game/Items/Collectatbles/S_Slot` _item))
        (:`NewEnumerator0`
          (return true))
        (:`NewEnumerator1`
          (if (< (`self.CurrentEquippedWeaponIndex`) 0)
            (`self.SetEquippedItem` (`local.Item`) (`local.Index`) :!label _label)))
        (:`NewEnumerator2`
          (if (< (`self.CurrentEquippedShieldIndex`) 0)
            (goto _label)
            (else
              _))))
      (return true)
      (elif (== _rowname (`.RowName` (break `DataTableRowHandle` (`.ItemID_4_80829AD24C0CEDA2206E46838C32E882` (break `/Game/Items/Collectatbles/S_Slot` (`local.Item`))))))
        (if (`|EnumEquality` (`.ItemType_9_26E7E05B4F92E22B1DD70092B75988D9` (break `/Game/Items/Collectatbles/S_Slot` (`local.Item`))) "NewEnumerator0")
          (bind _returnvalue (`|GetDataTableRow` "/Game/Items/Collectatbles/DT_CollectableItem.DT_CollectableItem" (`.RowName` (break `DataTableRowHandle` (`.ItemID_4_80829AD24C0CEDA2206E46838C32E882` (break `/Game/Items/Collectatbles/S_Slot` (`local.Item`))))))
            (:`then`
              (bind (_name _description _iconimage _statsize _numberininventory) (break `/Game/Items/Collectatbles/S_CollectableItem` _returnvalue))
              (if (> _numberininventory _quantity_2)
                (bind _returnvalue_2 (+ _quantity_2 1))
                (`KismetArrayLibrary.Array_Set` (`local.ItemArray`) (`local.Index`) (make `/Game/Items/Collectatbles/S_Slot` _itemid _returnvalue_2 _itemtype))
                (`KismetSystemLibrary.PrintString` (`KismetStringLibrary.Concat_StrStr` (`KismetStringLibrary.Conv_NameToString` _name) (`KismetStringLibrary.Conv_IntToString` _returnvalue_2)))
                (return true)
                (else
                  (return false)))))))))
  (if (`|EnumEquality` (`.ItemType_9_26E7E05B4F92E22B1DD70092B75988D9` (break `/Game/Items/Collectatbles/S_Slot` (`local.Item`))) "NewEnumerator0")
    (`self.ExpandInventory` (`local.ItemArray`))
    (`KismetArrayLibrary.Array_Set` (`local.ItemArray`) (- (`KismetArrayLibrary.Array_Length` (`local.ItemArray`)) 1) (`local.Item`))
    (return true)
    (else
      (return false))))

(fn `DecreaseHealth`
  (params (InDecreaseHealthPoint :type "Float (double-precision)"))
  (set `self.Health` (- (`self.Health`) InDecreaseHealthPoint))
  (`/Game/Widgets/WBP_HealthBar.UpdateHealthBar` (`self.WBP_HealthBar`))
  (`/Game/Widgets/WBP_HealthBar.UpdateHealthBar` (`/Game/Widgets/WBP_Inventory.WBP_HealthBar` (`self.WBP_InventoryWidget`))))

(fn `ExpandInventory`
  (params (ItemArray :type "Array of /Game/Items/Collectatbles/S_Slot Structure"))
  (`KismetArrayLibrary.Array_Resize` ItemArray (+ (`KismetArrayLibrary.Array_Length` ItemArray) 1)))

(fn `IncreaseHealth`
  (params (InIncreaseHealthPoint :type "Float (double-precision)"))
  (set `self.Health` (+ InIncreaseHealthPoint (`self.Health`)))
  (`/Game/Widgets/WBP_HealthBar.UpdateHealthBar` (`self.WBP_HealthBar`))
  (`/Game/Widgets/WBP_HealthBar.UpdateHealthBar` (`/Game/Widgets/WBP_Inventory.WBP_HealthBar` (`self.WBP_InventoryWidget`))))

(fn `InitHealthBar`
  (bind _returnvalue (`|CreateWidget` "/Game/Widgets/WBP_HealthBar.WBP_HealthBar_C"))
  (bind _output_get (set `self.WBP_HealthBar` _returnvalue))
  (`UserWidget.SetPositionInViewport` _output_get (30.0 30.0) true)
  (`UserWidget.AddToViewport` _output_get 0))

(fn `OnInventoryClost`
  (`Widget.SetVisibility` (`self.WBP_Interact`) "Visible")
  (`Widget.SetVisibility` (`self.WBP_HealthBar`) "Visible")
  (`self.Sort Inventory`))

(fn `OnInventoryOpen`
  (if (`Widget.IsInViewport` (`self.WBP_Interact`))
    (`Widget.RemoveFromParent` (`self.WBP_Interact`)))
  (`Widget.SetVisibility` (`self.WBP_Interact`) "Hidden")
  (`Widget.SetVisibility` (`self.WBP_HealthBar`) "Hidden")
  (`UserWidget.AddToViewport` (`self.WBP_InventoryWidget`) 0))

(fn `PickUpRupee`
  (params (OverlappedComponent :type "PrimitiveComponent Object Reference") (OtherActor :type "Actor Object Reference") (OtherComp :type "PrimitiveComponent Object Reference") (OtherBodyIndex :type Integer) (bFromSweep :type Boolean) (SweepResult :type "HitResult Structure (by ref)"))
  (bind _asbp_rupee (cast `/Game/Items/Rupees/BP_Rupee` OtherActor))
  (bind (_rupeetype_datatable _rupeetype_rowname) (break `DataTableRowHandle` (`/Game/Items/Rupees/BP_Rupee.RupeeType` _asbp_rupee)))
  (bind _returnvalue (`|GetDataTableRow` "/Game/Items/Rupees/DT_Rupee.DT_Rupee" _rupeetype_rowname)
    (:`then`
      (bind _output_get (set `self.RupeeAmount` (+ (`.Amount_6_66C4248A4A1415EE9293A38A69FD2CDB` (break `/Game/Items/Rupees/S_Rupee` _returnvalue)) (`self.RupeeAmount`))))
      (`KismetSystemLibrary.PrintString` (`KismetStringLibrary.Concat_StrStr` "Get rupee for: " (`KismetStringLibrary.Conv_IntToString` _output_get)))
      (`Actor.K2_DestroyActor` _asbp_rupee)
      (set `/Game/Widgets/WBP_Inventory.RupeeAmount` (`self.RupeeAmount`) (`self.WBP_InventoryWidget`))
      (return))))

(fn `ReduceItemFromInventory`
  (params (InCurrentSelectedItem :type "/Game/Items/Collectatbles/S_Slot Structure"))
  (switch `/Game/Enums/EnumItemType` (`.ItemType_9_26E7E05B4F92E22B1DD70092B75988D9` (break `/Game/Items/Collectatbles/S_Slot` InCurrentSelectedItem))
    (:`NewEnumerator0`
      (`self.ReduceItemFromItemArray` (`.Materials_11_A4C8D597405D82D79F98BAA9BD1B6C02` (break `/Game/Items/S_InventoryItems` (`self.InventoryItems`)))))
    (:`NewEnumerator1`
      (`self.ReduceItemFromItemArray` (`.Weapons_6_204640D1462B9325452B4492E2270A77` (break `/Game/Items/S_InventoryItems` (`self.InventoryItems`)))))
    (:`NewEnumerator2`
      (`self.ReduceItemFromItemArray` (`.Shields_9_97E983774B854D39919EFCBD26DFE85F` (break `/Game/Items/S_InventoryItems` (`self.InventoryItems`)))))))

(fn `ReduceItemFromItemArray`
  (params (InItemArray :type "Array of /Game/Items/Collectatbles/S_Slot Structure"))
  (bind _thirdpersoncharacter (`self.ThirdPersonCharacter`))
  (bind (_itemid _quantity _itemtype _isbeingequipped) (break `/Game/Items/Collectatbles/S_Slot` (`|GetArrayItem` InItemArray (`/Game/Widgets/WBP_Inventory.CurrentSelectedItemIndex` (`self.WBP_InventoryWidget`)))))
  (bind _returnvalue (- _quantity 1))
  (if _isbeingequipped
    (switch `/Game/Enums/EnumItemType` _itemtype
      (:`NewEnumerator1`
        (`/Game/ThirdPerson/Blueprints/BP_ThirdPersonCharacter.Unequipped Weapon` _thirdpersoncharacter)
        (set `self.CurrentEquippedWeaponIndex` -1))
      (:`NewEnumerator2`
        (`/Game/ThirdPerson/Blueprints/BP_ThirdPersonCharacter.Unequipped Shield` _thirdpersoncharacter)
        (set `self.CurrentEquippedShieldIndex` -1))))
  (if (== _returnvalue 0)
    (`KismetArrayLibrary.Array_Set` (`local.InItemArray`) (`/Game/Widgets/WBP_Inventory.CurrentSelectedItemIndex` (`self.WBP_InventoryWidget`)) (make `/Game/Items/Collectatbles/S_Slot` (struct) 0 _itemtype))
    (else
      (`KismetArrayLibrary.Array_Set` (`local.InItemArray`) (`/Game/Widgets/WBP_Inventory.CurrentSelectedItemIndex` (`self.WBP_InventoryWidget`)) (make `/Game/Items/Collectatbles/S_Slot` _itemid _returnvalue _itemtype)))))

(fn `SetEquippedItem`
  (params (InItem :type "/Game/Items/Collectatbles/S_Slot Structure") (InItemIndex :type Integer))
  (bind (_itemid _quantity _itemtype _isbeingequipped) (break `/Game/Items/Collectatbles/S_Slot` InItem))
  (bind _thirdpersoncharacter (`self.ThirdPersonCharacter`))
  (bind _initemindex (`local.InItemIndex`))
  (if _isbeingequipped
    (switch `/Game/Enums/EnumItemType` _itemtype
      (:`NewEnumerator1`
        (set `self.CurrentEquippedWeaponIndex` -1)
        (`/Game/ThirdPerson/Blueprints/BP_ThirdPersonCharacter.Unequipped Weapon` _thirdpersoncharacter)
        (`self.UpdateEquippedItemUI` "NewEnumerator1" :!label _label))
      (:`NewEnumerator2`
        (set `self.CurrentEquippedShieldIndex` -1)
        (`/Game/ThirdPerson/Blueprints/BP_ThirdPersonCharacter.Unequipped Shield` _thirdpersoncharacter)
        (`self.UpdateEquippedItemUI` "NewEnumerator2" :!label _label_2)))
    (else
      (switch `/Game/Enums/EnumItemType` _itemtype
        (:`NewEnumerator1`
          (set `self.CurrentEquippedWeaponIndex` _initemindex)
          (`/Game/ThirdPerson/Blueprints/BP_ThirdPersonCharacter.Equipped Weapon` (`self.ThirdPersonCharacter`) (`local.InItem`))
          (goto _label))
        (:`NewEnumerator2`
          (set `self.CurrentEquippedShieldIndex` _initemindex)
          (`/Game/ThirdPerson/Blueprints/BP_ThirdPersonCharacter.Equipped Shield` (`self.ThirdPersonCharacter`) (`local.InItem`))
          (goto _label_2))))))

(fn `Sort Inventory`
  (locals (CurrentIndex :type Integer) (TempSlot :type "/Game/Items/Collectatbles/S_Slot Structure"))
  (`|ExecutionSequence`
    (:`then_0`
      (`self.SortItemArray` (`.Weapons_6_204640D1462B9325452B4492E2270A77` (break `/Game/Items/S_InventoryItems` (`self.InventoryItems`)))))
    (:`then_1`
      (`self.SortItemArray` (`.Shields_9_97E983774B854D39919EFCBD26DFE85F` (break `/Game/Items/S_InventoryItems` (`self.InventoryItems`)))))
    (:`then_2`
      (`self.SortItemArray` (`.Materials_11_A4C8D597405D82D79F98BAA9BD1B6C02` (break `/Game/Items/S_InventoryItems` (`self.InventoryItems`)))))))

(fn `SortItemArray`
  (params (InItemArray :type "Array of /Game/Items/Collectatbles/S_Slot Structure"))
  (locals (CurrentIndex :type Integer) (LastIndex :type Integer) (TempSlot :type "/Game/Items/Collectatbles/S_Slot Structure"))
  (bind _output_get (set `local.LastIndex` (- (`KismetArrayLibrary.Array_Length` InItemArray) 1)))
  (for _index (range (+ _output_get 1))
    (bind _output_get_2 (set `local.CurrentIndex` _index))
    (for _ (range _output_get_2 (`KismetArrayLibrary.Array_Length` (`local.InItemArray`)))
      (if (!= (`local.CurrentIndex`) (`local.LastIndex`))
        (if (< (`.Quantity_6_B84E18094767D75D5B042897B33F25E0` (break `/Game/Items/Collectatbles/S_Slot` (`|GetArrayItem` (`local.InItemArray`) (`local.CurrentIndex`)))) (`.Quantity_6_B84E18094767D75D5B042897B33F25E0` (break `/Game/Items/Collectatbles/S_Slot` (`|GetArrayItem` (`local.InItemArray`) (+ (`local.CurrentIndex`) 1)))))
          (set `local.TempSlot` (`|GetArrayItem` (`local.InItemArray`) (`local.CurrentIndex`)))
          (`KismetArrayLibrary.Array_Set` (`local.InItemArray`) (`local.CurrentIndex`) (`|GetArrayItem` (`local.InItemArray`) (+ (`local.CurrentIndex`) 1)))
          (`KismetArrayLibrary.Array_Set` (`local.InItemArray`) (+ (`local.CurrentIndex`) 1) (`local.TempSlot`))
          (set `local.TempSlot` (struct)))))))

(fn `SpawnObject`
  (params (InItem :type "/Game/Items/Collectatbles/S_Slot Structure"))
  (bind (_itemid _quantity _itemtype) (break `/Game/Items/Collectatbles/S_Slot` InItem))
  (bind _thirdpersoncharacter (`self.ThirdPersonCharacter`))
  (`|SpawnActorFromClass` "/Game/Items/Collectatbles/BP_CollectableItem.BP_CollectableItem_C" (`KismetMathLibrary.Conv_VectorToTransform` (+ (* (`Actor.GetActorForwardVector` _thirdpersoncharacter) 100.0) (`Actor.K2_GetActorLocation` _thirdpersoncharacter))) "AdjustIfPossibleButAlwaysSpawn" "MultiplyWithRoot" null (make `/Game/Items/Collectatbles/S_Slot` _itemid 1 _itemtype) null))

(fn `TraceItemToPickUp`
  (returns (Found :type Boolean) (FoundItem :type "/Game/Items/Collectatbles/S_Slot Structure") (ItemActor :type "Actor Object Reference"))
  (bind _returnvalue (- (`Actor.K2_GetActorLocation` (`GameplayStatics.GetPlayerCharacter` 0)) (0.0 0.0 90.0)))
  (bind _outhit (`KismetSystemLibrary.SphereTraceSingle` _returnvalue _returnvalue 100.0 "TraceTypeQuery1"))
  (bind _asbp_collectable_item (cast `/Game/Items/Collectatbles/BP_CollectableItem` (`.HitActor` (`GameplayStatics.BreakHitResult` _outhit)))
    (:`then`
      (return true (`/Game/Items/Collectatbles/BP_CollectableItem.Item` _asbp_collectable_item) (`.HitActor` (`GameplayStatics.BreakHitResult` _outhit))))
    (:`CastFailed`
      (return false (struct) null))))

(fn `UpdateEquippedItemUI`
  (params (InItemArray :type "/Game/Enums/EnumItemType Enum" :default "NewEnumerator0"))
  (switch `/Game/Enums/EnumItemType` InItemArray
    (:`NewEnumerator1`
      (for (_array_element _array_index) (`.Weapons_6_204640D1462B9325452B4492E2270A77` (break `/Game/Items/S_InventoryItems` (`self.InventoryItems`)))
        (bind (_itemid _quantity _itemtype) (break `/Game/Items/Collectatbles/S_Slot` _array_element))
        (`KismetArrayLibrary.Array_Set` (`.Weapons_6_204640D1462B9325452B4492E2270A77` (break `/Game/Items/S_InventoryItems` (`self.InventoryItems`))) _array_index (make `/Game/Items/Collectatbles/S_Slot` _itemid _quantity _itemtype (== _array_index (`self.CurrentEquippedWeaponIndex`))))))
    (:`NewEnumerator2`
      (for (_array_element_2 _array_index_2) (`.Shields_9_97E983774B854D39919EFCBD26DFE85F` (break `/Game/Items/S_InventoryItems` (`self.InventoryItems`)))
        (bind (_itemid_2 _quantity_2 _itemtype_2) (break `/Game/Items/Collectatbles/S_Slot` _array_element_2))
        (`KismetArrayLibrary.Array_Set` (`.Shields_9_97E983774B854D39919EFCBD26DFE85F` (break `/Game/Items/S_InventoryItems` (`self.InventoryItems`))) _array_index_2 (make `/Game/Items/Collectatbles/S_Slot` _itemid_2 _quantity_2 _itemtype_2 (== _array_index_2 (`self.CurrentEquippedShieldIndex`))))))))